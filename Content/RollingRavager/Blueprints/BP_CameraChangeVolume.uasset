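; Overlap volume that repositions the camera of a BallPawn entering it, used in Rolling Ravager.
; On begin overlap it overwrites the pawn's CameraRelativeLocation, taking X and Y from its own settings and Z from a plane value offset by the volume's world position.
; A head-mounted display check selects separate VR or normal camera values.
; Nothing restores the previous position when the pawn leaves.
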(event EventBeginPlay)

(event EventActorBeginOverlap
  (params (OtherActor :type Actor%20Object%20Reference))
  (bind _camerarelativexy (Variables|Default|GetCameraRelativeXY))
  (bind _vrcamerarelativexy (Variables|Default|GetVRCameraRelativeXY))
  (bind _asball_pawn (Utilities|Casting|CastToBallPawn OtherActor))
  (if (Class|HeadMountedDisplayFunctionLibrary|IsHeadMountedDisplayEnabled)
    ;[1 1 1] VR camera
    (Variables|/Game/RollingRavager/Blueprints/BallPawn.BallPawn_C|SetCameraRelativeLocation _asball_pawn (Math|Vector|MakeVector (.x _vrcamerarelativexy) (.y _vrcamerarelativexy) (.z (+ (Variables|Default|GetVRCameraZPlane) (Transformation|GetActorLocation)))))
    (else
      ;[1 1 1] Normal camera
      (Variables|/Game/RollingRavager/Blueprints/BallPawn.BallPawn_C|SetCameraRelativeLocation _asball_pawn (Math|Vector|MakeVector (.x _camerarelativexy) (.y _camerarelativexy) (.z (+ (Variables|Default|GetCameraZPlane) (Transformation|GetActorLocation))))))))

(event EventTick
  (params (DeltaSeconds :type Float%20%28single-precision%29)))

(fn ConstructionScript)